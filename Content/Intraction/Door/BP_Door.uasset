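; BP_Door is an interactable door that shows its prompt only to a locally controlled CombinedCharExample overlapping its interaction box.
; Its interaction interface stores the interactor and supplies WBP_DoorWidget, then binds to the created widget's dispatcher, which currently just prints the selection.
; An authority-gated FlipFlop and timeline for swinging the door open and closed exists but is unconnected, and the Intractor RepNotify is empty.
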(event OnComponentBeginOverlap(IntractBox)
  (params (OverlappedComponent :type Primitive%20Component%20Object%20Reference) (OtherActor :type Actor%20Object%20Reference) (OtherComp :type Primitive%20Component%20Object%20Reference) (OtherBodyIndex :type Integer) (bFromSweep :type Boolean) (SweepResult :type Hit%20Result%20Structure%20%28by%20ref%29))
  (bind _ascombined_char_example (Utilities|Casting|CastToCombinedCharExample OtherActor))
  (if (Pawn|IsLocallyControlled _ascombined_char_example)
    (Development|SetHiddeninGame (Variables|Default|GetIntractionPromt) false true)))

(event OnComponentEndOverlap(IntractBox)
  (params (OverlappedComponent :type Primitive%20Component%20Object%20Reference) (OtherActor :type Actor%20Object%20Reference) (OtherComp :type Primitive%20Component%20Object%20Reference) (OtherBodyIndex :type Integer))
  (bind _ascombined_char_example (Utilities|Casting|CastToCombinedCharExample OtherActor))
  (if (Pawn|IsLocallyControlled _ascombined_char_example)
    (Development|SetHiddeninGame (Variables|Default|GetIntractionPromt) true true)))

(event Custom|WBPDispatcher_Event_0
  (params (SelectedIntraction :type Integer))
  (Development|PrintString (Utilities|String|Append "Selection ->" (Utilities|String|ToString(Integer) SelectedIntraction))))

(event EventBeginPlay
  (Development|SetHiddeninGame (Variables|Default|GetIntractionPromt) true true))

(event EventINTFIntractionWidgetCreated
  (params (NewParam :type User%20Widget%20Object%20Reference))
  (bind _aswbp_door_widget (Utilities|Casting|CastToWBP_DoorWidget NewParam))
  (EventDispatchers|AssignWBPDispatcher _aswbp_door_widget (delegate Custom|WBPDispatcher_Event_0)))

(fn ConstructionScript)

(fn OnRepIntractor)

(fn INTFIntraction
  (params (IntractorIn :type Combined%20Char%20Example%20Object%20Reference))
  (Variables|Default|SetIntractor IntractorIn)
  (return self "/Game/Intraction/Door/UIIntractionUI/WBP_DoorWidget.WBP_DoorWidget_C"))