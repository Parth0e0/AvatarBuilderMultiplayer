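; Base animal Blueprint that shows an interaction prompt and can play a paired handshake and graze animation with a player.
; A sphere overlap toggles the initially hidden prompt, only for a locally controlled CombinedCharExample.
; Multi_PlayAnim plays the handshake montage on the interacting character and the go-to-graze montage on the animal.
; The interaction interface function is empty, and the call to Multi_PlayAnim sits in unconnected logic that never runs.
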(event OnComponentBeginOverlap(Sphere)
  (params (OverlappedComponent :type Primitive%20Component%20Object%20Reference) (OtherActor :type Actor%20Object%20Reference) (OtherComp :type Primitive%20Component%20Object%20Reference) (OtherBodyIndex :type Integer) (bFromSweep :type Boolean) (SweepResult :type Hit%20Result%20Structure%20%28by%20ref%29))
  (bind _ascombined_char_example (Utilities|Casting|CastToCombinedCharExample OtherActor))
  (if (Pawn|IsLocallyControlled _ascombined_char_example)
    (Development|SetHiddeninGame (Variables|Default|GetIntractionPromt) false true)))

(event OnComponentEndOverlap(Sphere)
  (params (OverlappedComponent :type Primitive%20Component%20Object%20Reference) (OtherActor :type Actor%20Object%20Reference) (OtherComp :type Primitive%20Component%20Object%20Reference) (OtherBodyIndex :type Integer))
  (bind _ascombined_char_example (Utilities|Casting|CastToCombinedCharExample OtherActor))
  (if (Pawn|IsLocallyControlled _ascombined_char_example)
    (Development|SetHiddeninGame (Variables|Default|GetIntractionPromt) true true)))

(event Custom|Multi_PlayAnim
  (params (IntractorChar :type Combined%20Char%20Example%20Object%20Reference))
  (Animation|PlayAnimMontage IntractorChar "/Game/Maxamo/Mon_ShakeHand.Mon_ShakeHand" 1.0 "None")
  (Animation|PlayAnimMontage "/Game/Assets/AnimalVarietyPack/DeerStagAndDoe/Animations/Mon_GoToGraze.Mon_GoToGraze" 1.0 "None"))

(event EventBeginPlay
  (Development|SetHiddeninGame (Variables|Default|GetIntractionPromt) true true))

(fn ConstructionScript)

(fn INTFIntraction
  (return 0 0))