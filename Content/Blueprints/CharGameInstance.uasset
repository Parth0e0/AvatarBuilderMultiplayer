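; CharGameInstance is a game instance that stores character part selections and manages multiplayer session hosting and joining.
; Events save one set of parts and a separate set for all players, and a getter returns the former.
; Hosting creates a session through an Advanced Sessions node, then opens the Lobby level as a listen server on success.
; Joining passes a given search result to the session join node for the first player controller.
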(event Custom|StoreSavedParts
  (params (SavedParts :type S%20Saved%20Char%20Parts%20Structure))
  (Variables|Default|SetSavedParts SavedParts))

(event Custom|HostSession
  (|AdvancedSession 0 (Game|GetPlayerController 0) 100 0 false true false true true true false false false true false true
    (:OnSuccess
      (Game|OpenLevel(byName) "Lobby" true "?listen"))))

(event Custom|JoinSession
  (params (Session :type Blueprint%20Session%20Result%20Structure))
  (|JoinSession (Game|GetPlayerController 0) Session))

(event Custom|SaveAllPlayersParts
  (params (SavedParts :type Array%20of%20S%20Saved%20Char%20Parts%20Structures))
  (Variables|Default|SetSavedPlayerParts SavedParts))

(fn GetSavedParts
  (return (Variables|Default|GetSavedParts)))