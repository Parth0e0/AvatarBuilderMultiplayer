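; Modular customizable character that swaps clothing, hair, beard and sunglasses meshes and cycles their materials.
; Body part components follow the Head as master pose, set in the construction script.
; Add events toggle each part's mesh, while UpdateCharPart applies the next material from that part's array through a single Count index shared by all parts.
; SaveCharData stores current meshes and materials in SavedParts, which GetSavedParts returns.
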(event Custom|AddJacket
  (params (State :type Boolean))
  (bind _torso (Variables|Default|GetTorso))
  (if State
    (Class|SkinnedMeshComponent|SetSkeletalMesh _torso "/Game/SCK_Casual01/Models/MESH_T_01.MESH_T_01" true)
    (Rendering|Material|SetMaterial _torso 0 "/Game/SCK_Casual01/Materials/Material_Instances/Mi_T_01_1.Mi_T_01_1")
    (else
      (Class|SkinnedMeshComponent|SetSkeletalMesh _torso "/Game/SCK_Casual01/Models/MESH_T_00.MESH_T_00" true)
      (Rendering|Material|SetMaterial _torso 0 "/Game/SCK_Casual01/Materials/Master_Materials/MAT_T_00.MAT_T_00"))))

(event Custom|AddPants
  (params (State :type Boolean))
  (bind _legs (Variables|Default|GetLegs))
  (if State
    (Class|SkinnedMeshComponent|SetSkeletalMesh _legs "/Game/SCK_Casual01/Models/MESH_L_01.MESH_L_01" true)
    (Rendering|Material|SetMaterial _legs 0 "/Game/SCK_Casual01/Materials/Material_Instances/Mi_L_01_1.Mi_L_01_1")
    (else
      (Class|SkinnedMeshComponent|SetSkeletalMesh _legs "/Game/SCK_Casual01/Models/MESH_L_00.MESH_L_00" true)
      (Rendering|Material|SetMaterial _legs 0 "/Game/SCK_Casual01/Materials/Master_Materials/MAT_L_00.MAT_L_00"))))

(event Custom|AddHair
  (params (State :type Boolean) (NewMesh :type Skeletal%20Mesh%20Object%20Reference))
  (bind _hair (Variables|Default|GetHair))
  (if State
    (Class|SkinnedMeshComponent|SetSkeletalMesh _hair NewMesh true)
    (else
      (Class|SkinnedMeshComponent|SetSkeletalMesh _hair 0 true))))

(event Custom|AddSunglasses
  (params (State :type Boolean))
  (bind _sunglasses (Variables|Default|GetSunglasses))
  (if State
    (Class|SkinnedMeshComponent|SetSkeletalMesh _sunglasses "/Game/SCK_Casual01/Models/MESH_A_01.MESH_A_01" true)
    (else
      (Class|SkinnedMeshComponent|SetSkeletalMesh _sunglasses 0 true))))

(event Custom|AddBeard
  (params (State :type Boolean))
  (bind _beard (Variables|Default|GetBeard))
  (if State
    (Class|SkinnedMeshComponent|SetSkeletalMesh _beard "/Game/SCK_Casual01/Models/MESH_A_04.MESH_A_04" true)
    (else
      (Class|SkinnedMeshComponent|SetSkeletalMesh _beard 0 true))))

(event Custom|UpdateCharPart
  (params (UpdatePart :type E_CurrentCharPart%20Enum :default "NewEnumerator0"))
  (switch Utilities|FlowControl|Switch|SwitchonE_CurrentCharPart UpdatePart
    (:NewEnumerator1
      (bind _material (CallFunction|GetMaterial (Variables|Default|GetJacketMaterials)))
      (Rendering|Material|SetMaterial (Variables|Default|GetTorso) 0 _material))
    (:NewEnumerator2
      (bind _material_2 (CallFunction|GetMaterial (Variables|Default|GetPantsMaterials)))
      (Rendering|Material|SetMaterial (Variables|Default|GetLegs) 0 _material_2))
    (:NewEnumerator3
      (bind _material_3 (CallFunction|GetMaterial (Variables|Default|GetHair1Materials)))
      (Rendering|Material|SetMaterial (Variables|Default|GetHair) 0 _material_3))
    (:NewEnumerator6
      (bind _material_4 (CallFunction|GetMaterial (Variables|Default|GetHair2Materials)))
      (Rendering|Material|SetMaterial (Variables|Default|GetHair) 0 _material_4))
    (:NewEnumerator4
      (bind _material_5 (CallFunction|GetMaterial (Variables|Default|GetSunglassesMaterials)))
      (Rendering|Material|SetMaterial (Variables|Default|GetSunglasses) 0 _material_5))
    (:NewEnumerator5
      (bind _material_6 (CallFunction|GetMaterial (Variables|Default|GetBeardMaterials)))
      (Rendering|Material|SetMaterial (Variables|Default|GetBeard) 0 _material_6))))

(event Custom|SaveCharData
  (Utilities|Struct|SetmembersinS_SavedCharParts (Variables|Default|GetSavedParts) (Variables|/Script/Engine.SkinnedMeshComponent|GetSkeletalMesh (Variables|Default|GetTorso)) (Variables|/Script/Engine.SkinnedMeshComponent|GetSkeletalMesh (Variables|Default|GetLegs)) (Variables|/Script/Engine.SkinnedMeshComponent|GetSkeletalMesh (Variables|Default|GetHair)) (Variables|/Script/Engine.SkinnedMeshComponent|GetSkeletalMesh (Variables|Default|GetBeard)) (Variables|/Script/Engine.SkinnedMeshComponent|GetSkeletalMesh (Variables|Default|GetSunglasses)) (Utilities|Array|Get(acopy) (Rendering|Material|GetMaterials (Variables|Default|GetTorso))) (Utilities|Array|Get(acopy) (Rendering|Material|GetMaterials (Variables|Default|GetLegs))) (Utilities|Array|Get(acopy) (Rendering|Material|GetMaterials (Variables|Default|GetHair))) (Utilities|Array|Get(acopy) (Rendering|Material|GetMaterials (Variables|Default|GetSunglasses))) (Utilities|Array|Get(acopy) (Rendering|Material|GetMaterials (Variables|Default|GetBeard)))))

(fn ConstructionScript
  (Class|SkinnedMeshComponent|SetMasterPoseComponent (Variables|Default|GetLegs) (Variables|Default|GetHead) false))

(fn GetMaterial
  (params (IncomingMaterials :type Array%20of%20Material%20Interface%20Object%20References))
  (if (> (Variables|Default|GetCount) (- (Utilities|Array|Length IncomingMaterials) 1))
    (Variables|Default|SetCount 0)
    (else
      (Variables|Default|SetCount (+ (Variables|Default|GetCount) 1))))
  (return (Utilities|Array|Get(acopy) IncomingMaterials (Variables|Default|GetCount))))

(fn GetSavedParts
  (return (Variables|Default|GetSavedParts)))