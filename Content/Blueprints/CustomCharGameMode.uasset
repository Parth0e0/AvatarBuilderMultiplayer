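; Game mode for a multiplayer character customization stage that tracks joined players and starts the match when all are ready.
; A ready check polls each player's BP_CustomCharController, stops at the first unready one, and otherwise server-travels to LevelOne.
; Submitted character parts are stored at the matching player's index, then the whole array is saved to CharGameInstance.
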(event Custom|CheckIfPlayersReady
  (bind _readystate (Variables|Default|GetReadyState))
  (bind (_array_element _array_index) (Utilities|Array|ForEachLoopwithBreak (Variables|Default|GetConnectedPlayers) :!label _label)
    (:LoopBody
      (bind _asbp_custom_char_controller (Utilities|Casting|CastToBP_CustomCharController _array_element))
      (bind _ready (Default|GetReadyState _asbp_custom_char_controller))
      (if _ready
        (Utilities|Array|SetArrayElem _readystate _array_index true)
        (Variables|Default|SetCanStart true)
        (else
          (Utilities|Array|SetArrayElem _readystate _array_index false)
          (Variables|Default|SetCanStart false)
          (goto _label Break))))
    (:Completed
      (CallFunction|CanStartGame))))

(event Custom|CanStartGame
  (if (Variables|Default|GetCanStart)
    (Development|PrintString "ALL PLAYERS ARE READY" true true "(R=1.000000,G=0.000000,B=0.018907,A=1.000000)" 5.0)
    (Development|ExecuteConsoleCommand "servertravel LevelOne" (Game|GetPlayerController 0))
    (else
      (Development|PrintString "PLAYER NOT READY" true true "(R=1.000000,G=0.000000,B=0.018907,A=1.000000)" 5.0))))

(event Custom|SaveCharacterParts
  (params (Char :type S%20Saved%20Char%20Parts%20Structure) (PlayerController :type Player%20Controller%20Object%20Reference))
  (for (_array_element _array_index) (Variables|Default|GetConnectedPlayers)
    (if (== _array_element PlayerController)
      (Utilities|Array|SetArrayElem (Variables|Default|GetStoredParts) _array_index Char)))
  (bind _aschar_game_instance (Utilities|Casting|CastToCharGameInstance (Game|GetGameInstance)))
  (Default|SaveAllPlayersParts _aschar_game_instance (Variables|Default|GetStoredParts)))

(event EventPostLogin
  (params (NewPlayer :type Player%20Controller%20Object%20Reference))
  (Utilities|Array|AddUnique (Variables|Default|GetConnectedPlayers) NewPlayer))

(fn ConstructionScript)