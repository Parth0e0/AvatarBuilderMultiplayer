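; Game mode that hands each player controller the character parts saved in the game instance.
; On BeginPlay it caches SavedPlayerParts from CharGameInstance, and it adds controllers arriving through OnSwapPlayerControllers to a unique ConnectedPlayers list.
; GetSavedParts looks up a controller's position in that list and initializes its BP_GameController with the parts at the same index, so matching depends on arrival order.
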(event Custom|GetSavedParts
  (params (PC :type Player%20Controller%20Object%20Reference))
  (bind (_array_element _array_index) (Utilities|Array|ForEachLoopwithBreak (Variables|Default|GetConnectedPlayers) :!label _label)
    (:LoopBody
      (if (== _array_element PC)
        (goto _label Break)))
    (:Completed
      (bind _asbp_game_controller (Utilities|Casting|CastToBP_GameController PC))
      (Default|Initialize _asbp_game_controller (Utilities|Array|Get(acopy) (Variables|Default|GetSaved%20Player%20Parts) _array_index)))))

(event EventBeginPlay
  (bind _aschar_game_instance (Utilities|Casting|CastToCharGameInstance (Game|GetGameInstance)))
  (Variables|Default|SetSaved%20Player%20Parts (Variables|/Game/Blueprints/CharGameInstance.CharGameInstance_C|GetSavedPlayerParts _aschar_game_instance)))

(event EventOnSwapPlayerControllers
  (params (OldPC :type Player%20Controller%20Object%20Reference) (NewPC :type Player%20Controller%20Object%20Reference))
  (Utilities|Array|AddUnique (Variables|Default|GetConnectedPlayers) NewPC))

(fn ConstructionScript)