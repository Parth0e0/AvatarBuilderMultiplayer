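; Player controller for gameplay that applies saved character parts to the possessed pawn.
; After a one-second delay on possess, it passes itself to MainGameMode to request the saved parts.
; Its Initialize event hands received parts to CombinedCharExample for setup, then has the client clear all widgets and switch to game-only input.
; Escape quits the game.
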(event Custom|Initialize
  (params (Parts :type S%20Saved%20Char%20Parts%20Structure))
  (bind _ascombined_char_example (Utilities|Casting|CastToCombinedCharExample (Pawn|GetControlledPawn)))
  (Default|SetupCharacter _ascombined_char_example Parts)
  (CallFunction|ClientInitialize))

(event Custom|Client_Initialize
  (Viewport|RemoveAllWidgets)
  (Input|SetInputModeGameOnly self))

(event EventPossess
  (params (PossessedPawn :type Pawn%20Object%20Reference))
  (Utilities|FlowControl|Delay 1.0)
  (bind _asmain_game_mode (Utilities|Casting|CastToMainGameMode (Game|GetGameMode)))
  (Default|GetSavedParts _asmain_game_mode self))

(event Input|KeyboardEvents|Escape
  (params (Key :type Key%20Structure :default "None"))
  (:Pressed
    (Game|QuitGame 0 "Quit" false)))

(fn ConstructionScript)