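; Player controller for a networked character-creation screen where players customize a character, ready up and start.
; On BeginPlay it shows the W_BuildChar widget with UI-only input and caches the level's CustomCharacter, keeping the last one found.
; Part events forward clothing, hair and accessory changes to that character.
; Server events store readiness and, after a short post-save delay, pass saved parts to CustomCharGameMode, which also checks readiness.
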(event Custom|AddJacket
  (params (State :type Boolean))
  (Default|AddJacket (Variables|Default|GetCustomChar) State))

(event Custom|AddPants
  (params (State :type Boolean))
  (Default|AddPants (Variables|Default|GetCustomChar) State))

(event Custom|SaveSelectedChar
  (bind _customchar (Variables|Default|GetCustomChar))
  (Default|SaveCharData _customchar)
  (Utilities|FlowControl|Delay 0.2)
  (bind _savedpartsdata (Default|GetSavedParts _customchar))
  (CallFunction|ServerStorecharacter _savedpartsdata))

(event Custom|TryToStart
  (bind _ascustom_char_game_mode (Utilities|Casting|CastToCustomCharGameMode (Game|GetGameMode)))
  (Default|CheckifPlayersReady _ascustom_char_game_mode))

(event Custom|Server_Storecharacter
  (params (SavedParts :type S%20Saved%20Char%20Parts%20Structure))
  (bind _ascustom_char_game_mode (Utilities|Casting|CastToCustomCharGameMode (Game|GetGameMode)))
  (Default|SaveCharacterParts _ascustom_char_game_mode SavedParts self))

(event Custom|Client_DrawHud
  (bind _returnvalue (UserInterface|CreateWidget "/Game/Blueprints/W_BuildChar.W_BuildChar_C"))
  (bind _output_get (Variables|Default|SetCharBuildWidget _returnvalue))
  (UserInterface|Viewport|AddtoViewport _output_get 0)
  (Input|SetInputModeUIOnly self (Variables|Default|GetCharBuildWidget) "DoNotLock")
  (Variables|Default|SetbShowMouseCursor true))

(event Custom|AddHairStyle2
  (params (State :type Boolean))
  (Default|AddHair (Variables|Default|GetCustomChar) State "/Game/SCK_Casual01/Models/MESH_A_03.MESH_A_03"))

(event Custom|ReadyUp
  (params (Ready :type Boolean))
  (CallFunction|ServerReadyUp Ready))

(event Custom|AddHairStyle1
  (params (State :type Boolean))
  (Default|AddHair (Variables|Default|GetCustomChar) State "/Game/SCK_Casual01/Models/MESH_A_02.MESH_A_02"))

(event Custom|Server_ReadyUp
  (params (Ready :type Boolean))
  (Variables|Default|SetReady Ready))

(event Custom|AddSunglasses
  (params (State :type Boolean))
  (Default|AddSunglasses (Variables|Default|GetCustomChar) State))

(event Custom|AddBeard
  (params (State :type Boolean))
  (Default|AddBeard (Variables|Default|GetCustomChar) State))

(event Custom|UpdateCharPart
  (params (UpdateParts :type E_CurrentCharPart%20Enum :default "NewEnumerator0"))
  (Default|UpdateCharPart (Variables|Default|GetCustomChar) UpdateParts))

(event EventBeginPlay
  (bind _aschar_game_instance (Utilities|Casting|CastToCharGameInstance (Game|GetGameInstance)))
  (Variables|Default|SetGameInstance _aschar_game_instance)
  (Utilities|FlowControl|Sequence
    (:then_0
      (CallFunction|ClientDrawHud))
    (:then_1
      (bind _outactors (Actor|GetAllActorsOfClass "/Game/Blueprints/CustomCharacter.CustomCharacter_C"))
      (for _array_element _outactors
        (Variables|Default|SetCustomChar _array_element)))))

(event Input|KeyboardEvents|Escape
  (params (Key :type Key%20Structure :default "None"))
  (:Pressed
    (Game|QuitGame 0 "Quit" false)))

(fn ConstructionScript)

(fn GetReadyState
  (return (Variables|Default|GetReady)))